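; Game instance for a Pong game that holds both players' scores and a score-target-reached flag.
; A Reset event zeroes both scores and clears the flag.
; Separate increment events raise each player's score and apply modulo 10 to keep it a single digit.
; The flag is only cleared here, with no check against a target score in this graph.
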(event Custom|Reset
  ;[1 1 1] Clear player scores to zero and reset score target reached definition.
  (Variables|Default|SetPlayer1Score 0)
  (Variables|Default|SetPlayer2Score 0)
  (Variables|Default|SetScoreTargetReached false))

(event Custom|IncrementPlayer2Score
  ;[1 1 1] Increment the score for the player 2.
  (bind _result (Math|Integer|IncrementInt (Variables|Default|GetPlayer2Score))
    (:%20%20
      (Variables|Default|SetPlayer2Score (Math|Integer|%(Integer) _result 10)))))

(event Custom|IncrementPlayer1Score
  ;[1 1 1] Increment the score for the player 1.
  (bind _result (Math|Integer|IncrementInt (Variables|Default|GetPlayer1Score))
    (:%20%20
      (Variables|Default|SetPlayer1Score (Math|Integer|%(Integer) _result 10)))))