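; BasicSocketAgent is a socket client Blueprint that connects to a server and receives integer messages.
; ConnectToServer opens a connection to the given host on its Port variable, stores it on success and prints the status.
; ReceiveInt uses length-prefixed framing: it reads a fixed-size header giving the payload length, then reads and deserializes that payload as an integer.
; BeginPlay is empty, so nothing here starts the connection automatically.
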(event EventBeginPlay)

(fn ConstructionScript)

(fn ConnecttoServer
  (params (Host :type String))
  (Development|PrintString "Connecting to server...")
  (bind (_success _returnvalue) (Class|SocketerBPLibrary|Connect Host (Variables|Default|GetPort)))
  (if _success
    (Development|PrintString "Connection established")
    (Variables|Default|SetConnection _returnvalue)
    (else
      (Development|PrintString "Connection failed"))))

(fn ReceiveInt
  (bind _connection (Variables|Default|GetConnection))
  (bind _message (Class|SocketerBPLibrary|GetMessageFixedSize _connection 10))
  (bind _message_2 (Class|SocketerBPLibrary|GetMessageFixedSize _connection (Math|Conversions|ToInteger(Byte) _message)))
  (bind _returnvalue (Class|Serializer|DeserializeInt _message_2))
  (return _returnvalue))