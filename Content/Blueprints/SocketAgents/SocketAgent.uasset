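; SocketAgent is a reinforcement-learning style agent that exchanges observations, actions and rewards with a remote peer over a socket connection.
; Act serializes the float observation array, sends it over Connection, then returns the received integer as the chosen action.
; Learn sends the reward and the Done flag as two separate serialized integer messages, without reading a reply.
; The graphs here do not open the connection.
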(event EventBeginPlay
  (|CallParentFunction) ; This node is disabled and will not be called.\nDrag off pins to build functionality.
)

(fn ConstructionScript
  (|CallParentFunction))

(fn Act
  (params (Observations :type Array%20of%20Floats%20%28single-precision%29))
  ;[1 1 1] Send
  (bind _returnvalue (Class|Serializer|SerializeArrayFloat Observations))
  (Class|SocketerBPLibrary|SendMessage (Variables|Default|GetConnection) _returnvalue)
  ;[1 1 1] Recieve
  (bind _newparam (CallFunction|ReceiveInt))
  (return _newparam))

(fn Learn
  (params (Reward :type Integer) (done :type Boolean))
  (bind _connection (Variables|Default|GetConnection))
  (bind _returnvalue (Class|Serializer|SerializeInt Reward))
  (Class|SocketerBPLibrary|SendMessage _connection _returnvalue)
  (bind _returnvalue_2 (Class|Serializer|SerializeInt (Math|Conversions|ToInteger(Boolean) done)))
  (Class|SocketerBPLibrary|SendMessage _connection _returnvalue_2))